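; Moving platform actor that travels through an array of placed waypoint actors, with its mesh and material applied in the construction script.
; BeginPlay hides each waypoint in game and calls PlatformStart inside that loop, resetting to the first segment.
; A timeline lerps the actor's location between current and next waypoint positions.
; Timeline events advance to the next segment, or at path end restart from the first waypoint when Loop is set.
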(event `self.ReceiveBeginPlay`
  (for _array_element (`self.Waypoints`)
    (`self.SetActorHiddenInGame` _array_element true)
    (`self.Platform Start`)))

(event `Platform Start`
  (`self.Set_First_Waypoint`)
  (`TimelineComponent.PlayFromStart` (`self.Motion Timeline`)))

(fn `Path_Is_Finished`
  (returns (Is_Finished :type Boolean))
  (return (== (`self.Next_Waypoint_Index`) (- (`KismetArrayLibrary.Array_Length` (`self.Waypoints`)) 1))))

(fn `Set_First_Waypoint`
  (set `self.Current_Waypoint_Index` 0)
  (set `self.Next_Waypoint_Index` 1)
  (`self.Set_Positions`))

(fn `Set_Next_Waypoint`
  (bind _result (`/Engine/EditorBlueprintResources/StandardMacros.IncrementInt` (`self.Current_Waypoint_Index`))
    (:`  `
      (set `self.Next_Waypoint_Index` (+ _result 1))
      (`self.Set_Positions`))))

(fn `Set_Positions`
  (bind _waypoints (`self.Waypoints`))
  (set `self.Current_Waypoint_Position` (`self.K2_GetActorLocation` (`|GetArrayItem` _waypoints (`self.Current_Waypoint_Index`))))
  (set `self.Next_Waypoint_Position` (`self.K2_GetActorLocation` (`|GetArrayItem` _waypoints (`self.Next_Waypoint_Index`)))))

(fn `UserConstructionScript`
  (bind _platform_mesh (`self.Platform_Mesh`))
  (`StaticMeshComponent.SetStaticMesh` _platform_mesh (`self.Static_Mesh`))
  (`PrimitiveComponent.SetMaterial` _platform_mesh 0 (`self.Material`)))