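; MyGameManager is a game manager Blueprint that tracks the current game state and switches UI and mouse cursor to match it.
; Init creates the abandon widget, adds it to the viewport and enters the Running state.
; SetState hides the UI, stores the new state, then either hides the cursor for Running or reveals the widget and cursor for Abandon.
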(fn `Create UI`
  (bind _returnvalue (`|CreateWidget` "/Game/_MyContent/UI/Widget_Abandon.Widget_Abandon_C"))
  (bind _output_get (set `self.Widget_Abandon` _returnvalue))
  (`UserWidget.AddToViewport` _output_get 0))

(fn `Get State`
  (returns (State :type "/Game/_MyContent/Blueprints/MyGameStates Enum"))
  (return (`self.Current Game State`)))

(fn `Init`
  (`self.Create UI`)
  (`self.Set State` "NewEnumerator0"))

(fn `Set State`
  (params (`New State` :type "/Game/_MyContent/Blueprints/MyGameStates Enum" :default "NewEnumerator0"))
  (`/Game/_MyContent/Blueprints/MyFunctionLibrary.Hide UI`)
  (bind _output_get (set `self.Current Game State` `New State`))
  (switch `/Game/_MyContent/Blueprints/MyGameStates` _output_get
    (:`NewEnumerator0`
      (`/Game/_MyContent/Blueprints/MyFunctionLibrary.Show Mouse` false))
    (:`NewEnumerator2`
      (`Widget.SetVisibility` (`self.Widget_Abandon`) "Visible")
      (`/Game/_MyContent/Blueprints/MyFunctionLibrary.Show Mouse` true))))

(fn `UserConstructionScript`)